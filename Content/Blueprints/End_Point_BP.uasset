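; End_Point_BP is the goal trigger that plays an oven-style end sequence when a Turtle_Bot_BP reaches it.
; Its Box overlap casts to the turtle, waits briefly, then destroys it.
; A chain of timed delays then plays the Burn sound, spikes the RectLight intensity while activating Smoke, dims the light again and finally deactivates the smoke.
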(event `self.Box.OnComponentBeginOverlap`
  (params (OverlappedComponent :type "PrimitiveComponent Object Reference") (OtherActor :type "Actor Object Reference") (OtherComp :type "PrimitiveComponent Object Reference") (OtherBodyIndex :type Integer) (bFromSweep :type Boolean) (SweepResult :type "HitResult Structure (by ref)"))
  ;[1 1 1] When Turtle_BP begin overlap to Box Collision, starts end scenario
  (bind _asturtle_bot_bp (cast `/Game/Blueprints/Turtle/Turtle_Bot_BP` OtherActor))
  (`KismetSystemLibrary.Delay` 0.6)
  (`self.K2_DestroyActor` _asturtle_bot_bp)
  (`KismetSystemLibrary.Delay` 1.0)
  ;;[1 1 1] Play oven sound, set intensity to 10000, activate smoke particle
  (`AudioComponent.Play` (`self.Burn`) 0.0)
  (`KismetSystemLibrary.Delay` 0.65)
  (`LightComponent.SetIntensity` (`self.RectLight`) 10000.0)
  (`ActorComponent.Activate` (`self.Smoke`) false)
  (`KismetSystemLibrary.Delay` 2.4)
  ;;[1 1 1] Set intensity back to 1500, deactivate smoke particle
  (`LightComponent.SetIntensity` (`self.RectLight`) 1500.0)
  (`KismetSystemLibrary.Delay` 2.0)
  (`ActorComponent.Deactivate` (`self.Smoke`)))

(fn `UserConstructionScript`)